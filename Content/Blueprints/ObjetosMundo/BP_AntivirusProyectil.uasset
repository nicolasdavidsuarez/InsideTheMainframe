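; Antivirus projectile actor that hits third-person characters flagged as a virus.
; Tick moves it along its forward vector at constant speed on X and Y only, with a short lifespan set on BeginPlay.
; On sphere overlap with a virus character, it passes its forward direction to HitProyectil, activates a Niagara effect and destroys itself after a delay.
; Other overlaps are ignored, and movement continues during that delay.
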(event `self.ReceiveBeginPlay`
  (`self.SetLifeSpan` 3.0))

(event `self.ReceiveTick`
  (params (DeltaSeconds :type "Float (single-precision)"))
  (bind (_returnvalue_x _returnvalue_y) (`KismetMathLibrary.BreakVector` (`KismetMathLibrary.GetForwardVector` (`self.K2_GetActorRotation`))))
  (`self.K2_AddActorWorldOffset` (`KismetMathLibrary.MakeVector` (* _returnvalue_x DeltaSeconds 1000.0) (* DeltaSeconds _returnvalue_y 1000.0))))

(event `self.ReceiveActorBeginOverlap`
  (params (OtherActor :type "Actor Object Reference")))

(event `self.Sphere.OnComponentBeginOverlap`
  (params (OverlappedComponent :type "PrimitiveComponent Object Reference") (OtherActor :type "Actor Object Reference") (OtherComp :type "PrimitiveComponent Object Reference") (OtherBodyIndex :type Integer) (bFromSweep :type Boolean) (SweepResult :type "HitResult Structure (by ref)"))
  (bind _asbp_third_person_character (cast `/Game/Levels/Blueprints/BP_ThirdPersonCharacter` OtherActor))
  (if (`InsideTheMainframeCharacter.bIsVirus` _asbp_third_person_character)
    (`/Game/Levels/Blueprints/BP_ThirdPersonCharacter.HitProyectil` _asbp_third_person_character (`KismetMathLibrary.GetForwardVector` (`self.K2_GetActorRotation`)))
    (`ActorComponent.Activate` (`self.Niagara`) false)
    (`KismetSystemLibrary.Delay` 1.0)
    (`self.K2_DestroyActor`)))

(fn `UserConstructionScript`)