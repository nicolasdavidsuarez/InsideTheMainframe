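; BP_Capacitor is a world pickup station that recharges the third-person character on entering its box.
; When CoolDown is true, overlap spawns a charge Niagara effect before the character cast, calls RechargeFromCapacitor, clears the flag and deactivates the idle effect.
; Every overlap, even during cooldown, sets a short timer whose Enfriar event restores the flag and reactivates the effect.
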(event `self.Box.OnComponentBeginOverlap`
  (params (OverlappedComponent :type "PrimitiveComponent Object Reference") (OtherActor :type "Actor Object Reference") (OtherComp :type "PrimitiveComponent Object Reference") (OtherBodyIndex :type Integer) (bFromSweep :type Boolean) (SweepResult :type "HitResult Structure (by ref)"))
  (`KismetSystemLibrary.K2_SetTimerDelegate` (delegate `enfriar`) 2.0)
  (if (`self.CoolDown`)
    (`NiagaraFunctionLibrary.SpawnSystemAttached` "/Game/FX/NS_CapaciterCharge.NS_CapaciterCharge" (`self.NS_CapaciterCharge`) "None" (0.0 0.0 0.0) (struct) "KeepRelativeOffset")
    (bind _asbp_third_person_character (cast `/Game/Levels/Blueprints/BP_ThirdPersonCharacter` OtherActor))
    (`InsideTheMainframeCharacter.RechargeFromCapacitor` _asbp_third_person_character)
    (set `self.CoolDown` false)
    (`ActorComponent.Deactivate` (`self.Niagara`))))

(event `enfriar`
  (set `self.CoolDown` true)
  (`ActorComponent.Activate` (`self.Niagara`) false))

(fn `UserConstructionScript`)